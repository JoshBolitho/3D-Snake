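; Player pawn for the head of a 3D grid-based Snake game, steered along six directions by keys.
; A looping Delay steps it forward, spawning a BP_SnakeBodyActor behind with TimeToLive from BodySize, forming the tail.
; Steps and turns toggle CollisionWarning through TestImminentCollision, whose arena-bounds expression appears unconnected.
; Overlapping a body segment opens GameOverMenu, while Fruit overlaps are ignored here.
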(event `self.ReceiveActorBeginOverlap`
  (params (OtherActor :type "Actor Object Reference"))
  (cast `/Game/Blueprints/Fruit` OtherActor
    (:`CastFailed`
      (cast `/Game/Blueprints/BP_SnakeBodyActor` OtherActor)
      (bind _returnvalue (`|CreateWidget` "/Game/Blueprints/Menus/GameOverMenu.GameOverMenu_C"))
      (`UserWidget.AddToViewport` _returnvalue 0))))

(event `self.ReceiveBeginPlay`
  (`self.K2_SetActorRotation` (`KismetMathLibrary.MakeRotator` 0.0 0.0 180.0) true)
  (set `self.PrevTransform` (`self.GetTransform`) :!label _label)
  (`self.K2_AddActorWorldOffset` (* (`self.GetActorForwardVector`) 105))
  (`GameplayStatics.PlaySound2D` "/Game/Audio/Pop_Cue.Pop_Cue" 1.0 1.0 0.0 null null)
  (if (`self.TestImminentCollision`)
    (`SceneComponent.SetVisibility` (`self.collision warning`) true true)
    (else
      (`SceneComponent.SetVisibility` (`self.collision warning`) false true)))
  (bind _returnvalue (`|SpawnActorFromClass` "/Game/Blueprints/BP_SnakeBodyActor.BP_SnakeBodyActor_C" (`self.PrevTransform`) "Undefined" "OverrideRootScale" null null))
  (set `/Game/Blueprints/BP_SnakeBodyActor.TimeToLive` (`self.BodySize`) _returnvalue)
  (`KismetSystemLibrary.Delay` 0.5)
  (goto _label))

(event `Key|W`
  (params (Key :type "Key Structure"))
  (:`Pressed`
    (`self.K2_SetActorRotation` (`KismetMathLibrary.MakeRotator` 0.0) true :!label _label_2)
    (if (`self.TestImminentCollision`) :!label _label_3
      (`SceneComponent.SetVisibility` (`self.collision warning`) true true)
      (else
        (`SceneComponent.SetVisibility` (`self.collision warning`) false true)))))

(event `Key|Up`
  (params (Key :type "Key Structure"))
  (:`Pressed`
    (goto _label_2)))

(event `Key|S`
  (params (Key :type "Key Structure"))
  (:`Pressed`
    (`self.K2_SetActorRotation` (`KismetMathLibrary.MakeRotator` 0.0 0.0 180.0) true :!label _label_4)
    (goto _label_3)))

(event `Key|Down`
  (params (Key :type "Key Structure"))
  (:`Pressed`
    (goto _label_4)))

(event `Key|A`
  (params (Key :type "Key Structure"))
  (:`Pressed`
    (`self.K2_SetActorRotation` (`KismetMathLibrary.MakeRotator` 0.0 0.0 270.0) true :!label _label_5)
    (goto _label_3)))

(event `Key|Left`
  (params (Key :type "Key Structure"))
  (:`Pressed`
    (goto _label_5)))

(event `Key|D`
  (params (Key :type "Key Structure"))
  (:`Pressed`
    (`self.K2_SetActorRotation` (`KismetMathLibrary.MakeRotator` 0.0 0.0 90.0) true :!label _label_6)
    (goto _label_3)))

(event `Key|Right`
  (params (Key :type "Key Structure"))
  (:`Pressed`
    (goto _label_6)))

(event `Key|PageUp`
  (params (Key :type "Key Structure"))
  (:`Pressed`
    (`self.K2_SetActorRotation` (`KismetMathLibrary.MakeRotator` 0.0 90.0) true)
    (`self.K2_SetActorRelativeRotation` (`KismetMathLibrary.MakeRotator` 0.0 90.0 180.0))
    (goto _label_3)))

(event `Key|PageDown`
  (params (Key :type "Key Structure"))
  (:`Pressed`
    (`self.K2_SetActorRotation` (`KismetMathLibrary.MakeRotator` 0.0 -90.0) true)
    (`self.K2_SetActorRelativeRotation` (`KismetMathLibrary.MakeRotator` 180.0 270.0))
    (goto _label_3)))

(fn `UserConstructionScript`
  (locals (BodyLength :type Integer))
  (set `local.BodyLength` 1))
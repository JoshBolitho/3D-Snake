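; Game mode for a Snake game that provides StartGame and EndGame functions to begin and finish a round.
; StartGame shows the snake head, adds fade and HUD widgets, resets body size, jump time and head rotation, and enables input.
; EndGame hides the head with an explosion, destroys body actors and shows the game-over menu with UI-only input.
; Both set the GameRunning flag on SnakeGameInstance.
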(event `self.ReceiveBeginPlay`)

(fn `EndGame`
  ;[1 1 1] End Game
  (bind _assnake_game_instance (cast `/Game/Blueprints/SnakeGameInstance` (`GameplayStatics.GetGameInstance`)))
  (set `/Game/Blueprints/SnakeGameInstance.GameRunning` false _assnake_game_instance)
  ;[1 1 1] Hide Snake Head
  (`SceneComponent.SetVisibility` (`Actor.RootComponent` (`GameplayStatics.GetPlayerPawn` 0)) false true)
  ;[1 1 1] Explode Head
  (`GameplayStatics.SpawnEmitterAtLocation` "/Game/StarterContent/Particles/P_Explosion.P_Explosion" (`self.K2_GetActorLocation` (`GameplayStatics.GetPlayerPawn` 0)) (struct) (10.0 10.0 10.0))
  (`GameplayStatics.PlaySound2D` "/Game/StarterContent/Audio/Explosion_Cue.Explosion_Cue" 1.0 1.0 0.0 null null)
  ;[1 1 1] Hide Snake Body
  (bind _outactors (`GameplayStatics.GetAllActorsOfClass` "/Game/Blueprints/BP_SnakeBodyActor.BP_SnakeBodyActor_C"))
  (for _array_element _outactors
    (`self.K2_DestroyActor` _array_element))
  ;[1 1 1] Add Game Over Screen
  (bind _returnvalue (`|CreateWidget` "/Game/Blueprints/UI/GameOverMenu.GameOverMenu_C"))
  (`UserWidget.AddToViewport` _returnvalue 0)
  ;[1 1 1] Disable Input
  (`WidgetBlueprintLibrary.SetInputMode_UIOnlyEx` (`GameplayStatics.GetPlayerController` 0) _returnvalue "LockAlways"))

(fn `StartGame`
  ;[1 1 1] Show Snake Head
  (`SceneComponent.SetVisibility` (`Actor.RootComponent` (`GameplayStatics.GetPlayerPawn` 0)) true true)
  ;[1 1 1] Hide Cursor
  (set `PlayerController.bShowMouseCursor` false (`GameplayStatics.GetPlayerController` 0))
  ;[1 1 1] Fade In Animation
  (bind _returnvalue (`|CreateWidget` "/Game/Blueprints/UI/Fade.Fade_C" (`GameplayStatics.GetPlayerController` 0)))
  (`UserWidget.AddToViewport` _returnvalue 0)
  ;[1 1 1] Add HUD
  (bind _returnvalue_2 (`|CreateWidget` "/Game/Blueprints/UI/HUD.HUD_C" (`GameplayStatics.GetPlayerController` 0)))
  (bind _output_get (set `self.HUD` _returnvalue_2))
  (`UserWidget.AddToViewport` _output_get 0)
  ;[1 1 1] Reset Game Parameters
  (bind _assnake_game_instance (cast `/Game/Blueprints/SnakeGameInstance` (`GameplayStatics.GetGameInstance`)))
  (set `/Game/Blueprints/SnakeGameInstance.Body_Size` 2 _assnake_game_instance)
  (set `/Game/Blueprints/SnakeGameInstance.Jump_Time` 0.35 _assnake_game_instance)
  (bind _asbp_snake_head_pawn (cast `/Game/Blueprints/BP_SnakeHeadPawn` (`GameplayStatics.GetPlayerPawn` 0)))
  (`self.K2_SetActorLocationAndRotation` _asbp_snake_head_pawn (0.0 0.0 0.0) (`KismetMathLibrary.MakeRotator` 0.0 0.0 180.0) false false)
  ;[1 1 1] Enable Input
  (`WidgetBlueprintLibrary.SetInputMode_GameAndUIEx` (`GameplayStatics.GetPlayerController` 0) null)
  ;[1 1 1] Set Global Game Running Parameter
  (bind _assnake_game_instance_2 (cast `/Game/Blueprints/SnakeGameInstance` (`GameplayStatics.GetGameInstance`)))
  (set `/Game/Blueprints/SnakeGameInstance.GameRunning` true _assnake_game_instance_2))

(fn `UserConstructionScript`)
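; Fruit is a collectible actor that grows a body size counter when overlapped, apparently food for a snake-style game.
; Any actor overlap increments BodySize on MyGameInstance, with no check on which actor touched it.
; It then spawns a replacement Fruit at a random cell on a bounded 3D grid around the world origin, plays a chomp sound and destroys itself.
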(event `self.ReceiveActorBeginOverlap`
  (params (OtherActor :type "Actor Object Reference"))
  (bind _asmy_game_instance (cast `/Game/Blueprints/MyGameInstance` (`GameplayStatics.GetGameInstance`)))
  (bind _result (`/Engine/EditorBlueprintResources/StandardMacros.IncrementInt` (`/Game/Blueprints/MyGameInstance.Body_Size` _asmy_game_instance))
    (:`  `
      (set `/Game/Blueprints/MyGameInstance.Body_Size` _result _asmy_game_instance)
      (`|SpawnActorFromClass` "Fruit_C" (`KismetMathLibrary.MakeTransform` (`KismetMathLibrary.MakeVector` (* (`KismetMathLibrary.RandomIntegerInRange` -7 7) 105.0) (* (`KismetMathLibrary.RandomIntegerInRange` -7 7) 105.0) (* (`KismetMathLibrary.RandomIntegerInRange` -7 7) 105.0))) "Undefined" "OverrideRootScale" null null)
      (`GameplayStatics.PlaySound2D` "/Game/Audio/chomp_Cue.chomp_Cue" 1.0 1.0 0.0 null null)
      (`self.K2_DestroyActor`))))

(fn `UserConstructionScript`)